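; RTS camera pawn that pans, zooms and rotates an orthographic camera over a bounded map.
; Axis input and optional screen-edge mouse panning feed movement input along the YawPivot's flattened forward and right vectors, so panning follows camera yaw.
; Rotate actions step the pivot yaw, zoom adjusts clamped OrthoWidth, and FastPan swaps the FloatingPawnMovement speed, acceleration and deceleration.
; Tick clamps the actor's XY position to the configured limits.
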(event `InputAction|FastPan`
  (params (Key :type "Key Structure"))
  (bind _floatingpawnmovement (`self.FloatingPawnMovement`))
  (:`Pressed`
    (set `FloatingPawnMovement.MaxSpeed` (`self.FastPanSpeed`) _floatingpawnmovement)
    (set `FloatingPawnMovement.Acceleration` (`self.FastAccel `) _floatingpawnmovement)
    (set `FloatingPawnMovement.Deceleration` (`self.FastDecel `) _floatingpawnmovement))
  (:`Released`
    (set `FloatingPawnMovement.MaxSpeed` (`self.BasePanSpeed`) _floatingpawnmovement)
    (set `FloatingPawnMovement.Acceleration` (`self.BaseAccel `) _floatingpawnmovement)
    (set `FloatingPawnMovement.Deceleration` (`self.BaseDecel`) _floatingpawnmovement)))

(event `self.ReceiveBeginPlay`
  (bind _yawpivot (`self.YawPivot`))
  (bind _floatingpawnmovement (`self.FloatingPawnMovement`))
  (`|ExecutionSequence`
    (:`then_0`
      (bind _output_get (set `self.CameraYaw` (.yaw (`SceneComponent.RelativeRotation` _yawpivot))))
      (`SceneComponent.K2_SetRelativeRotation` _yawpivot (`KismetMathLibrary.MakeRotator` 0.0 0.0 _output_get) false false))
    (:`then_1`
      (set `FloatingPawnMovement.MaxSpeed` (`self.BasePanSpeed`) _floatingpawnmovement)
      (set `FloatingPawnMovement.Acceleration` (`self.BaseAccel `) _floatingpawnmovement)
      (set `FloatingPawnMovement.Deceleration` (`self.BaseDecel`) _floatingpawnmovement))))

(event `InputAxis|MoveForward`
  (params (AxisValue :type "Float (single-precision)"))
  (`self.AddMovementInput` (`KismetMathLibrary.Normal` (`KismetMathLibrary.MakeVector` (.x (`SceneComponent.GetForwardVector` (`self.YawPivot`))) (.y (`SceneComponent.GetForwardVector` (`self.YawPivot`))))) AxisValue))

(event `InputAxis|MoveRight`
  (params (AxisValue :type "Float (single-precision)"))
  (`self.AddMovementInput` (`KismetMathLibrary.Normal` (`KismetMathLibrary.MakeVector` (.x (`SceneComponent.GetRightVector` (`self.YawPivot`))) (.y (`SceneComponent.GetRightVector` (`self.YawPivot`))))) AxisValue))

(event `InputAxis|Zoom`
  (params (AxisValue :type "Float (single-precision)"))
  (bind _camera (`self.Camera`))
  (set `CameraComponent.OrthoWidth` (`KismetMathLibrary.FClamp` (- (`CameraComponent.OrthoWidth` _camera) (* AxisValue (`self.ZoomStep`))) (`self.MinOrthoWidth`) (`self.MaxOrthoWidth`)) _camera))

(event `InputAction|RotateLeft`
  (params (Key :type "Key Structure"))
  (:`Pressed`
    (bind _output_get (set `self.CameraYaw` (- (`self.CameraYaw`) (`self.RotateStep`))))
    (`SceneComponent.K2_SetRelativeRotation` (`self.YawPivot`) (`KismetMathLibrary.MakeRotator` 0.0 0.0 _output_get) false false)))

(event `InputAction|RotateRight`
  (params (Key :type "Key Structure"))
  (:`Pressed`
    (bind _output_get (set `self.CameraYaw` (+ (`self.CameraYaw`) (`self.RotateStep`))))
    (`SceneComponent.K2_SetRelativeRotation` (`self.YawPivot`) (`KismetMathLibrary.MakeRotator` 0.0 0.0 _output_get) false false)))

(event `self.ReceiveTick`
  (params (DeltaSeconds :type "Float (single-precision)"))
  (bind _returnvalue (`GameplayStatics.GetPlayerController` 0))
  (bind (_sizex _sizey) (`PlayerController.GetViewportSize` _returnvalue))
  (bind (_locationx _locationy _returnvalue_2) (`PlayerController.GetMousePosition` _returnvalue))
  (bind _returnvalue_3 (* (`self.EdgePanSpeed`) (`GameplayStatics.GetWorldDeltaSeconds`)))
  (`|ExecutionSequence`
    (:`then_1`
      (if (`self.EdgePanEnabled`)
        (if _returnvalue_2
          (`|ExecutionSequence`
            (:`then_0`
              (if (<= _locationx (`self.EdgePanBorderPx`))
                (`self.AddMovementInput` (`KismetMathLibrary.Normal` (`KismetMathLibrary.MakeVector` (.x (* (`SceneComponent.GetRightVector` (`self.YawPivot`)) (`KismetMathLibrary.Conv_DoubleToVector` -1.0))) (.y (* (`SceneComponent.GetRightVector` (`self.YawPivot`)) (`KismetMathLibrary.Conv_DoubleToVector` -1.0))))) _returnvalue_3)))
            (:`then_1`
              (if (>= _locationx (- _sizex (`self.EdgePanBorderPx`)))
                (`self.AddMovementInput` (`KismetMathLibrary.Normal` (`KismetMathLibrary.MakeVector` (.x (`SceneComponent.GetRightVector` (`self.YawPivot`))) (.y (`SceneComponent.GetRightVector` (`self.YawPivot`))))) _returnvalue_3)))
            (:`then_2`
              (if (>= _locationy (- _sizey (`self.EdgePanBorderPx`)))
                (`self.AddMovementInput` (`KismetMathLibrary.Normal` (`KismetMathLibrary.MakeVector` (.x (* (`SceneComponent.GetForwardVector` (`self.YawPivot`)) (`KismetMathLibrary.Conv_DoubleToVector` -1.0))) (.y (* (`SceneComponent.GetForwardVector` (`self.YawPivot`)) (`KismetMathLibrary.Conv_DoubleToVector` -1.0))))) _returnvalue_3)))
            (:`then_3`
              (if (<= _locationy (`self.EdgePanBorderPx`))
                (`self.AddMovementInput` (`KismetMathLibrary.Normal` (`KismetMathLibrary.MakeVector` (.x (`SceneComponent.GetForwardVector` (`self.YawPivot`))) (.y (`SceneComponent.GetForwardVector` (`self.YawPivot`))))) _returnvalue_3)))))))
    (:`then_2`
      (`self.K2_SetActorLocation` (`KismetMathLibrary.MakeVector` (`KismetMathLibrary.FClamp` (.x (`self.K2_GetActorLocation`)) (`self.MinX`) (`self.MaxX`)) (`KismetMathLibrary.FClamp` (.y (`self.K2_GetActorLocation`)) (`self.MinY`) (`self.MaxY`)) (.z (`self.K2_GetActorLocation`)))))))

(fn `UserConstructionScript`)